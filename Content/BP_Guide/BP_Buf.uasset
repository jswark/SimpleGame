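; BP_Buf is an actor with a Buf component whose look is randomized, apparently an unfinished buff or trap.
; The construction script rolls 0 to 2 to pick one of two materials, leaving the default on the third outcome.
; BeginPlay caches the first BP_PlayerState.
; Overlap sets a timer with no function name given, and TrapOverlapping is empty, so no gameplay effect is implemented.
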(event EventBeginPlay
  (bind _asbp_player_state (Utilities|Casting|CastToBP_PlayerState (Game|GetPlayerState 0)))
  (Variables|Default|SetMy%20Player%20State _asbp_player_state))

(event Collision|EventActorBeginOverlap
  (params (OtherActor :type Actor%20Object%20Reference))
  (Utilities|Time|SetTimerbyFunctionName 0 "" 5.0))

(event EventTick
  (params (DeltaSeconds :type Float%20%28single-precision%29)))

(fn ConstructionScript
  (switch int (Math|Random|RandomIntegerinRange 0 2)
    (:0
      (Rendering|Material|SetMaterial (Variables|Default|GetBuf) 0 "/Game/StarterContent/Materials/M_ColorGrid_LowSpec.M_ColorGrid_LowSpec"))
    (:1
      (Rendering|Material|SetMaterial (Variables|Default|GetBuf) 0 "/Game/StarterContent/Props/Materials/M_MaterialSphere.M_MaterialSphere"))))

(fn TrapOverlapping)