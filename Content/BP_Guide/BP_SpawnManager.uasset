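; BP_SpawnManager populates each new room with randomly placed traps and walls.
; On BeginPlay it caches the player state and binds both spawn events to the game mode's new-room event.
; Each event reads its count from the player state and spawns BP_Trap or BP_Walls at random floor positions within fixed bounds, with walls adjusted to avoid collisions where possible.
; SpawnBufs is an empty stub.
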(event Custom|Spawn%20Traps
  (params (CurrentRoom :type Integer))
  (for _index (range 0 (Variables|/Game/ThirdPerson/Blueprints/BP_PlayerState.BP_PlayerState_C|GetTrapAmount (Variables|Default|GetMy%20Player%20State)))
    (Game|SpawnActorfromClass "/Game/BP_Guide/BP_Trap.BP_Trap_C" (Math|Conversions|ToTransform(Vector) (Math|Vector|MakeVector (Math|Random|RandomFloatinRange 6.8e+02 2.84e+03) (Math|Random|RandomFloatinRange 1.2e+02 3.35e+03) 0.0)) "Undefined" 0 0)))

(event Custom|Spawn%20Bufs
  (params (Amount :type Integer)))

(event Custom|Spawn%20Wall
  (params (CurrentRoom :type Integer))
  (for _index (range 0 (Variables|/Game/ThirdPerson/Blueprints/BP_PlayerState.BP_PlayerState_C|GetWallAmount (Variables|Default|GetMy%20Player%20State)))
    (Game|SpawnActorfromClass "/Game/BP_Guide/BP_Walls.BP_Walls_C" (Math|Conversions|ToTransform(Vector) (Math|Vector|MakeVector (Math|Random|RandomFloatinRange 3.2e+02 2.04e+03) (Math|Random|RandomFloatinRange 1.2e+02 3.35e+03) 0.0)) "AdjustIfPossibleButAlwaysSpawn" 0 0)))

(event EventBeginPlay
  (bind _asbp_player_state (Utilities|Casting|CastToBP_PlayerState (Game|GetPlayerState 0)))
  (Variables|Default|SetMy%20Player%20State _asbp_player_state)
  (bind _asbp_guide_gamemode (Utilities|Casting|CastToBP_Guide_Gamemode (Game|GetGameMode)))
  (EventDispatchers|BindEventtoNewRoom _asbp_guide_gamemode (delegate Custom|Spawn%20Traps))
  (EventDispatchers|BindEventtoNewRoom _asbp_guide_gamemode (delegate Custom|Spawn%20Wall)))

(event Collision|EventActorBeginOverlap
  (params (OtherActor :type Actor%20Object%20Reference)))

(event EventTick
  (params (DeltaSeconds :type Float%20%28single-precision%29)))

(fn ConstructionScript)