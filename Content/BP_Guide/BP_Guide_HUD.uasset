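; BP_Guide_HUD is a HUD that shows the player's score, time and level, plus a game over screen.
; On BeginPlay it casts player state 0 to BP_PlayerState and caches it.
; DrawHUD draws colored text labels along the top of the screen from that state each frame.
; When the state's GameOver flag is set, it also draws GAME OVER and PRESS ENTER prompts.
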(event EventBeginPlay
  (bind _asbp_player_state (Utilities|Casting|CastToBP_PlayerState (Game|GetPlayerState 0)))
  (Variables|Default|SetMy_Player_State _asbp_player_state))

(event Collision|EventActorBeginOverlap
  (params (OtherActor :type Actor%20Object%20Reference)))

(event EventTick
  (params (DeltaSeconds :type Float%20%28single-precision%29)))

(event EventDrawHUD
  (params (SizeX :type Integer) (SizeY :type Integer))
  (HUD|DrawText (Utilities|String|BuildString(Integer) "Score" "" (Variables|/Game/BP_Guide/BP_PlayerState.BP_PlayerState_C|GetScore1 (Variables|Default|GetMy_Player_State))) "(R=1.000000,G=0.940253,B=0.144000,A=1.000000)" 1e+01 1e+01 0 3.0 false)
  (HUD|DrawText (Utilities|String|BuildString(Integer) "Time" "" (Variables|/Game/BP_Guide/BP_PlayerState.BP_PlayerState_C|GetTime (Variables|Default|GetMy_Player_State))) "(R=0.488000,G=0.000000,B=0.082534,A=1.000000)" 3e+02 1e+01 0 3.0 false)
  (HUD|DrawText (Utilities|String|BuildString(Integer) "Player Level" "" (Variables|/Game/BP_Guide/BP_PlayerState.BP_PlayerState_C|GetLevel (Variables|Default|GetMy_Player_State))) "(R=0.134330,G=0.132000,B=1.000000,A=1.000000)" 5.5e+02 1e+01 0 3.0 false)
  (if (Variables|/Game/BP_Guide/BP_PlayerState.BP_PlayerState_C|GetGameOver (Variables|Default|GetMy_Player_State))
    (HUD|DrawText "GAME OVER" "(R=0.552000,G=0.000000,B=0.000000,A=1.000000)" 4e+02 2e+02 0 3.0 false)
    (HUD|DrawText "PRESS ENTER" "(R=0.732000,G=0.000000,B=0.000000,A=1.000000)" 4e+02 4e+02 0 3.0 false)))

(fn ConstructionScript)