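; BP_Trap is a hazard actor that calls TrapOverlap on the guide game mode when the player character overlaps it.
; The construction script randomly makes it Dynamic or Static, with one roll leaving the default Type.
; Dynamic traps move their mesh every tick, bouncing between Y bounds at the player state's TrapSpeed without delta-time scaling.
; They also creep along negative X and destroy themselves below zero.
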(event Custom|Move%20Trap
  (bind _staticmesh (Variables|Default|GetStaticMesh))
  (bind _returnvalue (Transformation|GetWorldLocation _staticmesh))
  (bind (_x _y) (Class|KismetMathLibrary|BreakVector3f _returnvalue))
  (Transformation|SetWorldLocation (Variables|Default|GetStaticMesh) (+ (Transformation|GetWorldLocation (Variables|Default|GetStaticMesh)) (Math|Vector|MakeVector -0.005 (Math|Conversions|ToFloat(Integer) (* (Variables|/Game/ThirdPerson/Blueprints/BP_PlayerState.BP_PlayerState_C|GetTrapSpeed (Variables|Default|GetMy%20PlayerState)) (Variables|Default|Getforward))) 0.0)) false false)
  (if (> _y 3.35e+03)
    (Variables|Default|Setforward -1))
  (if (< _y 1.2e+02)
    (Variables|Default|Setforward 1))
  (if (< _x 0.0)
    (Actor|DestroyActor)))

(event EventBeginPlay
  (bind _asbp_guide_gamemode (Utilities|Casting|CastToBP_Guide_Gamemode (Game|GetGameMode)))
  (Variables|Default|SetMy%20GameMode _asbp_guide_gamemode)
  (bind _asbp_player_state (Utilities|Casting|CastToBP_PlayerState (Game|GetPlayerState 0)))
  (Variables|Default|SetMy%20PlayerState _asbp_player_state)
  (if (> (.Y (Class|KismetMathLibrary|BreakVector3f (Transformation|GetWorldLocation (Variables|Default|GetStaticMesh)))) 3.35e+03)
    (Variables|Default|Setforward -1)
    (else
      (Variables|Default|Setforward 1))))

(event Collision|EventActorBeginOverlap
  (params (OtherActor :type Actor%20Object%20Reference))
  (if (== OtherActor (Game|GetPlayerCharacter 0))
    (Default|TrapOverlap (Variables|Default|GetMy%20GameMode))))

(event EventTick
  (params (DeltaSeconds :type Float%20%28single-precision%29))
  (switch Utilities|FlowControl|Switch|SwitchonE_TrapType (Variables|Components|GetType)
    (:NewEnumerator0
      (CallFunction|MoveTrap))))

(fn ConstructionScript
  (switch int (Math|Random|RandomIntegerinRange 0 2)
    (:0
      (Variables|Components|SetType "NewEnumerator0"))
    (:1
      (Variables|Components|SetType "NewEnumerator1"))))