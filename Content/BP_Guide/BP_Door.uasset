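; BP_Door is a door actor that reports to the guide game mode when the player walks into it, flagging whether it is a heal room door.
; Its Type enum sets the HealRoom flag passed to the game mode's DoorOverlap.
; The construction script gives heal room doors a different material.
; BeginPlay caches the game mode and player state, though the player state is unused here.
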(event EventBeginPlay
  (bind _asbp_guide_gamemode (Utilities|Casting|CastToBP_Guide_Gamemode (Game|GetGameMode)))
  (Variables|Default|SetMyGuideGameMode _asbp_guide_gamemode)
  (bind _asbp_player_state (Utilities|Casting|CastToBP_PlayerState (Game|GetPlayerState 0)))
  (Variables|Default|SetMyPlayerState _asbp_player_state))

(event Collision|EventActorBeginOverlap
  (params (OtherActor :type Actor%20Object%20Reference))
  (if (== OtherActor (Game|GetPlayerCharacter 0))
    (switch Utilities|FlowControl|Switch|SwitchonE_DoorType (Variables|Components|GetType)
      (:NewEnumerator0
        (Variables|Default|SetHealRoom false))
      (:NewEnumerator1
        (Variables|Default|SetHealRoom true)))
    (Default|DoorOverlap (Variables|Default|GetMyGuideGameMode) (Variables|Default|GetHealRoom))))

(event EventTick
  (params (DeltaSeconds :type Float%20%28single-precision%29)))

(fn ConstructionScript
  (switch Utilities|FlowControl|Switch|SwitchonE_DoorType (Variables|Components|GetType)
    (:NewEnumerator1
      (Rendering|Material|SetMaterial (Variables|Default|GetDoor) 0 "/Game/StarterContent/Materials/M_ColorGrid_LowSpec.M_ColorGrid_LowSpec"))))