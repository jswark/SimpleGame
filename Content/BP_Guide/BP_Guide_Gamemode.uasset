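; BP_Guide_Gamemode is the game mode for a timed statue-collecting game, keeping all round state in BP_PlayerState.
; StartGame resets that state and starts a looping one-second Clock timer, which sets GameOver and stops when time hits exactly zero.
; StatueCollected applies level-scaled score or a time bonus or penalty, raising the capped level every fifth statue.
; RestartGame reuses the BeginPlay path.
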(event Custom|Clock
  (bind _my_player_state (Variables|Default|GetMy%20Player%20State))
  (Variables|/Game/BP_Guide/BP_PlayerState.BP_PlayerState_C|SetTime _my_player_state (- (Variables|/Game/BP_Guide/BP_PlayerState.BP_PlayerState_C|GetTime _my_player_state) 1))
  (if (== (Variables|/Game/BP_Guide/BP_PlayerState.BP_PlayerState_C|GetTime _my_player_state) 0)
    (Variables|/Game/BP_Guide/BP_PlayerState.BP_PlayerState_C|SetGameOver _my_player_state true)
    (Utilities|Time|ClearTimerbyFunctionName 0 "Clock")))

(event Custom|Restart%20Game
  (bind _asbp_player_state (Utilities|Casting|CastToBP_PlayerState (Game|GetPlayerState 0)))
  (Variables|Default|SetMy%20Player%20State _asbp_player_state)
  (Utilities|StartGame))

(event EventTick
  (params (DeltaSeconds :type Float%20%28single-precision%29)))

(event EventBeginPlay
  (bind _asbp_player_state (Utilities|Casting|CastToBP_PlayerState (Game|GetPlayerState 0)))
  (Variables|Default|SetMy%20Player%20State _asbp_player_state)
  (Utilities|StartGame))

(fn ConstructionScript)

(fn StatueCollected
  (params (BonusType :type E_BonusType%20Enum :default "NewEnumerator0"))
  (bind _my_player_state (Variables|Default|GetMy%20Player%20State))
  (bind _my_player_state_2 (Variables|Default|GetMy%20Player%20State))
  (bind _my_player_state_3 (Variables|Default|GetMy%20Player%20State))
  (switch Utilities|FlowControl|Switch|SwitchonE_BonusType BonusType
    (:NewEnumerator0
      (Variables|/Game/BP_Guide/BP_PlayerState.BP_PlayerState_C|SetScore1 _my_player_state_3 (+ (Variables|/Game/BP_Guide/BP_PlayerState.BP_PlayerState_C|GetScore1 _my_player_state_3) (* (Variables|/Game/BP_Guide/BP_PlayerState.BP_PlayerState_C|GetLevel _my_player_state_3) 10))))
    (:NewEnumerator1
      (Variables|/Game/BP_Guide/BP_PlayerState.BP_PlayerState_C|SetTime _my_player_state_3 (+ (Variables|/Game/BP_Guide/BP_PlayerState.BP_PlayerState_C|GetTime _my_player_state_3) 15)))
    (:NewEnumerator2
      (Variables|/Game/BP_Guide/BP_PlayerState.BP_PlayerState_C|SetTime _my_player_state_3 (+ (Variables|/Game/BP_Guide/BP_PlayerState.BP_PlayerState_C|GetTime _my_player_state_3) -15))))
  (Variables|/Game/BP_Guide/BP_PlayerState.BP_PlayerState_C|SetStatueCount _my_player_state_2 (+ (Variables|/Game/BP_Guide/BP_PlayerState.BP_PlayerState_C|GetStatueCount _my_player_state_2) 1))
  (if (== (Math|Integer|%(Integer) (Variables|/Game/BP_Guide/BP_PlayerState.BP_PlayerState_C|GetStatueCount _my_player_state_2) 5) 0)
    (Variables|/Game/BP_Guide/BP_PlayerState.BP_PlayerState_C|SetLevel _my_player_state (Math|Integer|Min(Integer) (+ (Variables|/Game/BP_Guide/BP_PlayerState.BP_PlayerState_C|GetLevel _my_player_state) 1) 5))))