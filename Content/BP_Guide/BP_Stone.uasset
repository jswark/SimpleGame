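; BP_Stone is a pickup actor that heals through the game mode when the player touches it.
; On BeginPlay it caches references to BP_Guide_Gamemode and the first player's BP_PlayerState.
; Overlap with the player character calls the game mode's Heal and destroys the stone.
; Tick polls the player state's HealRoom flag and destroys the stone whenever that flag is false.
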(event EventBeginPlay
  (bind _asbp_guide_gamemode (Utilities|Casting|CastToBP_Guide_Gamemode (Game|GetGameMode)))
  (Variables|Default|SetMy%20GameMode _asbp_guide_gamemode)
  (bind _asbp_player_state (Utilities|Casting|CastToBP_PlayerState (Game|GetPlayerState 0)))
  (Variables|Default|SetMy%20PlayerState _asbp_player_state))

(event Collision|EventActorBeginOverlap
  (params (OtherActor :type Actor%20Object%20Reference))
  (if (== (Game|GetPlayerCharacter 0) OtherActor)
    (Default|Heal (Variables|Default|GetMy%20GameMode))
    (Actor|DestroyActor)))

(event EventTick
  (params (DeltaSeconds :type Float%20%28single-precision%29))
  (if (== (Variables|/Game/ThirdPerson/Blueprints/BP_PlayerState.BP_PlayerState_C|GetHealRoom (Variables|Default|GetMy%20PlayerState)) false)
    (Actor|DestroyActor)))

(fn ConstructionScript)