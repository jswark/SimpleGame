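; BP_Statue is a spinning pickup that randomly becomes a score, plus-time or minus-time statue, with a matching material.
; InitStatue teleports it to a random spot in a fixed area and sets a timer to repeat, using the player state's Level minus six as delay.
; Player overlap, unless the game is over, reports the type to the guide game mode, bobs the statue, then destroys it and spawns a replacement.
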(event EventBeginPlay
  (bind _asbp_guide_gamemode (Utilities|Casting|CastToBP_Guide_Gamemode (Game|GetGameMode)))
  (Variables|Default|SetMy%20Guide%20Gamemode _asbp_guide_gamemode)
  (bind _asbp_player_state (Utilities|Casting|CastToBP_PlayerState (Game|GetPlayerState 0)))
  (Variables|Default|SetMy%20Player%20State _asbp_player_state)
  (CallFunction|InitStatue))

(event Collision|EventActorBeginOverlap
  (params (OtherActor :type Actor%20Object%20Reference))
  (if (and (== OtherActor (Game|GetPlayerCharacter 0)) (not (Variables|/Game/ThirdPerson/Blueprints/BP_PlayerState.BP_PlayerState_C|GetGameOver (Variables|Default|GetMy%20Player%20State))))
    (Default|StatueCollected (Variables|Default|GetMy%20Guide%20Gamemode) (Variables|Components|GetType))
    (Transformation|SetActorLocation (+ (Transformation|GetActorLocation) "0,0,50.000000") false false)
    (Utilities|FlowControl|Delay 0.2)
    (Transformation|SetActorLocation (+ (Transformation|GetActorLocation) "0,0,-50.000000") false false)
    (Utilities|FlowControl|Delay 0.2)
    (Actor|DestroyActor)
    (Variables|Components|SetType "NewEnumerator2")
    (Game|SpawnActorfromClass "BP_Statue_C" (Transformation|GetActorTransform) "Undefined" 0 0)))

(event EventTick
  (params (DeltaSeconds :type Float%20%28single-precision%29))
  (Transformation|AddRelativeRotation (Variables|Default|GetStatue) (Math|Rotator|MakeRotator 0.0 0.0 (* DeltaSeconds 1e+02)) false false))

(fn ConstructionScript
  (switch int (Math|Random|RandomIntegerinRange 0 2)
    (:0
      (Variables|Components|SetType "NewEnumerator0"))
    (:1
      (bind _output_get (Variables|Components|SetType "NewEnumerator1")))
    (:2
      (Variables|Components|SetType "NewEnumerator2")))
  (switch Utilities|FlowControl|Switch|SwitchonE_BonusType _output_get
    (:NewEnumerator0
      (Rendering|Material|SetMaterial (Variables|Default|GetStatue) 0 "/Game/StarterContent/Materials/M_Brick_Clay_Old.M_Brick_Clay_Old"))
    (:NewEnumerator1
      (Rendering|Material|SetMaterial (Variables|Default|GetStatue) 0 "/Game/LevelPrototyping/Materials/MI_Solid_Blue.MI_Solid_Blue"))
    (:NewEnumerator2
      (Rendering|Material|SetMaterial (Variables|Default|GetStatue) 0 "/Game/StarterContent/Props/Materials/M_TableRound.M_TableRound"))))

(fn InitStatue
  (Transformation|Teleport (Math|Vector|MakeVector (Math|Random|RandomFloatinRange 1e+02 1e+03) (Math|Random|RandomFloatinRange 1e+02 1.4e+03) 1.3e+02) "0, 0, 0")
  (Utilities|Time|SetTimerbyFunctionName 0 "Init Statue" (Math|Conversions|ToFloat(Integer) (- (Variables|/Game/ThirdPerson/Blueprints/BP_PlayerState.BP_PlayerState_C|GetLevel (Variables|Default|GetMy%20Player%20State)) 6))))